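; EffectsManager spawns Niagara effects when turtles are summoned or escape.
; On BeginPlay it binds to the GameManager's OnTurtleSummon and OnTurtleEscape dispatchers.
; Each handler spawns the same NS_Healing_3 system, at the indexed nest for a summon and at the indexed safe zone for an escape.
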(event `self.ReceiveBeginPlay`
  (bind _gamemanager (`self.GameManager`))
  ;[1 1 1] При старте подпишемся на события создания и уничтожения черепашек
  (add `/Game/Blueprints/GameManager.OnTurtleSummon` _gamemanager (delegate `PlaySummonEffect`))
  (add `/Game/Blueprints/GameManager.OnTurtleEscape` _gamemanager (delegate `PlayEscapeEffect`)))

(event `PlaySummonEffect`
  (params (Idx :type Integer))
  ;[1 1 1] При старте подпишемся на события создания и уничтожения черепашек
  (`NiagaraFunctionLibrary.SpawnSystemAtLocation` "/Game/VFX/NS_Healing_3.NS_Healing_3" (`self.K2_GetActorLocation` (`|GetArrayItem` (`self.Nests`) Idx)) (struct) (1.0 1.0 1.0) true true "None" false))

(event `PlayEscapeEffect`
  (params (Idx :type Integer) (Turtle :type "Actor Object Reference"))
  ;[1 1 1] При старте подпишемся на события создания и уничтожения черепашек
  (`NiagaraFunctionLibrary.SpawnSystemAtLocation` "/Game/VFX/NS_Healing_3.NS_Healing_3" (`self.K2_GetActorLocation` (`|GetArrayItem` (`self.SafeZones`) Idx)) (struct) (1.0 1.0 1.0) true true "None" false))

(fn `UserConstructionScript`)