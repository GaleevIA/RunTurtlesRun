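; TurtlesManager is an actor that spawns, moves and removes the turtles in the game.
; It listens to GameManager events: summon spawns a Turtle at the indexed nest and records that index on it, while escape unregisters and destroys it.
; Every Tick it calls Move on each tracked turtle, passing DeltaSeconds added to TurtleSpeed rather than multiplied by it.
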(event `self.ReceiveBeginPlay`
  (bind _gamemanager (`self.GameManager`))
  (add `/Game/Blueprints/GameManager.OnTurtleSummon` _gamemanager (delegate `SummonTurtle`))
  (add `/Game/Blueprints/GameManager.OnTurtleEscape` _gamemanager (delegate `DestroyTurtle`)))

(event `SummonTurtle`
  (params (Idx :type Integer))
  (`self.fSummonTurtle` Idx))

(event `DestroyTurtle`
  (params (Idx :type Integer) (Turtle :type "Actor Object Reference"))
  (bind _asturtle (cast `/Game/Blueprints/Turtle` Turtle))
  (`KismetArrayLibrary.Array_RemoveItem` (`self.Turtles`) _asturtle)
  (`self.K2_DestroyActor` Turtle))

(event `self.ReceiveTick`
  (params (DeltaSeconds :type "Float (single-precision)"))
  (for _array_element (`self.Turtles`)
    (`/Game/Blueprints/Turtle.Move` _array_element (+ DeltaSeconds (`self.TurtleSpeed`)))))

(fn `fSummonTurtle`
  (params (Idx :type Integer))
  (bind _returnvalue (`|SpawnActorFromClass` "/Game/Blueprints/Turtle.Turtle_C" (`self.GetTransform` (`|GetArrayItem` (`self.Nests`) Idx)) "Undefined" "OverrideRootScale" null null))
  (`KismetArrayLibrary.Array_Add` (`self.Turtles`) _returnvalue)
  (set `/Game/Blueprints/Turtle.NestIdx` Idx _returnvalue))

(fn `UserConstructionScript`)