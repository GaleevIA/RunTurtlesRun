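; Turtle actor that moves along world X in one of three patterns, chosen by the nest it spawned from.
; From BeginPlay, self-restarting one-shot timers toggle IsNotMove, alternating a longer interval with a shorter one.
; Move applies a Speed offset per call: nest 0 always advances, nest 1 pauses while IsNotMove is set, and nest 2 reverses instead.
; Tick is unused, so Move relies on an external caller.
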(event `self.ReceiveBeginPlay`
  ;[1 1 1] При создании черепашки запускаем цикл из 2 таймеров для реализации разного алгоритма перемещения. Через 1 секунду срабатывает событие, которое устанавливает состояние IsNotMove в ложь и запускает второй таймер. Через 0.5 секунды срабатывает событие, которое устанавливает состояние IsNotMove в истина и запускает первый таймер. Таким образом черепашка сама определяет свое текущее состояние.
  (`KismetSystemLibrary.K2_SetTimerDelegate` (delegate `ChangeMoveState`) (+ (`GameplayStatics.GetWorldDeltaSeconds`) 1.0) :!label _label))

(event `ChangeMoveState`
  ;[1 1 1] При создании черепашки запускаем цикл из 2 таймеров для реализации разного алгоритма перемещения. Через 1 секунду срабатывает событие, которое устанавливает состояние IsNotMove в ложь и запускает второй таймер. Через 0.5 секунды срабатывает событие, которое устанавливает состояние IsNotMove в истина и запускает первый таймер. Таким образом черепашка сама определяет свое текущее состояние.
  (bind _output_get (set `self.IsNotMove` (not (`self.IsNotMove`))))
  (if _output_get
    (`KismetSystemLibrary.K2_SetTimerDelegate` (delegate `ChangeMoveState`) (+ (`GameplayStatics.GetWorldDeltaSeconds`) 0.5))
    (else
      (goto _label))))

(fn `Move`
  (params (Speed :type "Float (double-precision)"))
  (bind _isnotmove (`self.IsNotMove`))
  ;[1 1 1] В зависимости от текущего состояния черепашка либо движется вперед, либо отрабатывает один из двух алгоритмов: стоит на месте и движется назад, в зависимости от гнезда, из которого она появилась.
  (switch `int` (`self.NestIdx`)
    (:`0`
      (`self.K2_AddActorWorldOffset` (`KismetMathLibrary.MakeVector` Speed) :!label _label))
    (:`1`
      (if (not _isnotmove)
        (goto _label)))
    (:`2`
      (if _isnotmove
        (`self.K2_AddActorWorldOffset` (`KismetMathLibrary.MakeVector` (* Speed -1.0)))
        (else
          (goto _label))))))

(fn `UserConstructionScript`)