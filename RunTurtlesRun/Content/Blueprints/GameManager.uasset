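; GameManager is the hub that relays turtle summon and escape events between the UI, the SafePlace actors and any listeners.
; On BeginPlay it creates the Interface widget, binds its summon button, and binds the overlap event of each actor in SafePlaces.
; Button presses rebroadcast as OnTurtleSummon with an index.
; Overlaps broadcast OnTurtleEscape with the safe place's array index and the overlapping actor as the turtle.
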(event `self.ReceiveBeginPlay`
  (bind _returnvalue (`|CreateWidget` "/Game/Blueprints/UMG/Interface.Interface_C"))
  (`UserWidget.AddToViewport` _returnvalue 0)
  (add `/Game/Blueprints/UMG/Interface.OnSummonButtonPress` _returnvalue (delegate `TurtleSummon`))
  (for _array_element (`self.SafePlaces`)
    (add `self.OnActorBeginOverlap` _array_element (delegate `TurtleEscape`))))

(event `TurtleEscape` :!signature `self.OnActorBeginOverlap`
  (params (OverlappedActor :type "Actor Object Reference") (OtherActor :type "Actor Object Reference"))
  (bind _assafe_place (cast `/Game/Blueprints/SafePlace` OverlappedActor))
  (`self.OnTurtleEscape` (`KismetArrayLibrary.Array_Find` (`self.SafePlaces`) _assafe_place) OtherActor))

(event `TurtleSummon`
  (params (Idx :type Integer))
  (`self.OnTurtleSummon` Idx))

(fn `UserConstructionScript`)